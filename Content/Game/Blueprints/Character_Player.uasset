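; Player character driven by a queue of commands read from the tags of a drag-to slot in the HUD it creates.
; ReadActions steps through the tags with a delayed loop macro, one per second, teleporting a fixed step forward or turning 90 degrees.
; Reset restores the starting transform and briefly ignores moves and turns, without cancelling the running loop.
; The T key prints the queued tags.
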(event `self.ReceiveBeginPlay`
  (`self.EnableInput` (`GameplayStatics.GetPlayerController` 0))
  (set `self.InitialLocation` (`self.K2_GetActorLocation` self))
  (bind _output_get (set `self.InitialRot` (`self.K2_GetActorRotation` self)))
  (set `self.PlayerRot` _output_get)
  (bind _returnvalue (`|CreateWidget` "/Game/Game/Blueprints/HUD.HUD_C"))
  (bind _output_get_2 (set `self.Widget_Ref` _returnvalue))
  (`UserWidget.AddToViewport` _output_get_2 0)
  (set `PlayerController.bShowMouseCursor` true (`GameplayStatics.GetPlayerController` 0)))

(event `MoveForward`
  (bind _returnvalue (`self.K2_GetActorLocation` self))
  ;[1 1 1] Movement / Rotations
  (if (not (`self.Reseted?`))
    (`self.K2_TeleportTo` (`KismetMathLibrary.VLerp` _returnvalue (+ _returnvalue (* (`self.GetActorForwardVector`) 110)) 1.0) (`self.PlayerRot`))))

(event `ReadActions`
  ;[1 1 1] Execute Actions
  (bind _arrayelement (`self.ForEachLoopWithDelay` (`/Game/Game/Blueprints/DragTo_W.Tags` (`/Game/Game/Blueprints/HUD.DragTo_W_157` (`self.Widget_Ref`))) 1.0)
    (:`Loop Body`
      (switch `string` _arrayelement
        (:`Forward`
          (`self.MoveForward`))
        (:`RotateRight`
          (`self.Rotate` 90.0))
        (:`RotateLeft`
          (`self.Rotate` -90.0))))))

(event `Rotate`
  (params (Direction :type "Float (double-precision)"))
  (bind (_returnvalue_roll _returnvalue_pitch _returnvalue_yaw) (`KismetMathLibrary.BreakRotator` (`self.K2_GetActorRotation` self)))
  ;[1 1 1] Movement / Rotations
  (if (not (`self.Reseted?`))
    (`self.K2_SetActorRotation` (`KismetMathLibrary.MakeRotator` 0.0 0.0 (+ _returnvalue_yaw Direction)))
    (set `self.PlayerRot` (`self.K2_GetActorRotation` self))))

(event `Reset`
  ;[1 1 1] Reset
  (set `self.Reseted?` true)
  (`self.K2_SetActorRotation` (`self.InitialRot`))
  (`self.K2_SetActorLocation` (`self.InitialLocation`))
  (set `self.PlayerRot` (`self.InitialRot`))
  (`KismetSystemLibrary.Delay` 0.5)
  (set `self.Reseted?` false))

(event `Key|T`
  (params (Key :type "Key Structure" :default "AnyKey"))
  (:`Pressed`
    (bind _arrayelement (`self.ForEachLoopWithDelay` (`/Game/Game/Blueprints/DragTo_W.Tags` (`/Game/Game/Blueprints/HUD.DragTo_W_157` (`self.Widget_Ref`))))
      (:`Loop Body`
        (`KismetSystemLibrary.PrintString` _arrayelement)))))

(fn `UserConstructionScript`)